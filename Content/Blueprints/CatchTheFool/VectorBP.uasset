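; VectorBP is an actor that wanders continuously between random points on a fixed-height plane.
; On BeginPlay it picks a destination in a square world-space area, then each Tick moves toward it by normalized direction, Speed and DeltaSeconds, without sweeping for collision.
; It picks a new destination once the remaining distance is less than Speed, roughly one second of travel before arrival.
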(event `self.ReceiveBeginPlay`
  (`self.SetRandomDestination`))

(event `self.ReceiveTick`
  (params (DeltaSeconds :type "Float (single-precision)"))
  (set `self.DeltaSeconds` DeltaSeconds)
  (set `self.vDistance` (- (`self.vDestination`) (`self.K2_GetActorLocation`)))
  (set `self.vDirection` (`KismetMathLibrary.Normal` (`self.vDistance`)))
  (set `self.vVelocity` (* (`self.vDirection`) (`self.Speed`)))
  (bind _output_get (set `self.vStep` (* (`self.vVelocity`) (`self.DeltaSeconds`))))
  (`self.K2_AddActorWorldOffset` _output_get)
  (if (< (`KismetMathLibrary.VSize` (`self.vDistance`)) (`self.Speed`))
    (`self.SetRandomDestination`)))

(fn `UserConstructionScript`)