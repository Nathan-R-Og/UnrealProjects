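; Game mode for a timed statue collection game that tracks score, level, remaining time and game-over state.
; StartGame runs on BeginPlay and RestartGame, resetting the state, starting a looping one-second Clock timer and calling NewGame.
; Clock counts down and ends the game when time runs out.
; StatueCollected adds level-scaled points, and every fifth statue grants bonus time and raises the level.
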(event `self.ReceiveBeginPlay`
  (`self.StartGame` :!label _label))

(event `RestartGame`
  (goto _label))

(event `Clock`
  (bind _time (`self.Time`))
  (`/Engine/EditorBlueprintResources/StandardMacros.DecrementInt` _time
    (:`  `
      (if (<= _time 0)
        (set `self.GameOver` true)
        (`KismetSystemLibrary.K2_ClearTimer` null "Clock")))))

(fn `StatueCollected`
  (bind _statuecount (`self.StatueCount`))
  (set `self.Score` (+ (`self.Score`) (* 10 (`self.Level`))))
  (`/Engine/EditorBlueprintResources/StandardMacros.IncrementInt` _statuecount
    (:`  `
      (if (== (mod _statuecount 5) 0)
        (set `self.Time` (+ (`self.Time`) 15))
        (`/Engine/EditorBlueprintResources/StandardMacros.IncrementInt` (`self.Level`))))))

(fn `UserConstructionScript`)