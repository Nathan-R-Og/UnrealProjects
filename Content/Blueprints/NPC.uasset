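; NPC Blueprint that shows a text widget on screen and hands it to a scene component, likely for dialogue.
; DoTextStuff runs only when the CScene class is valid, creating a Text widget for the first player controller and adding it visibly to the viewport.
; It then adds a CScene component at runtime and calls its Load with that widget.
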(fn `DoTextStuff`
  (locals (NewLocalVar :type "/Game/Blueprints/Text Object Reference"))
  (if (`KismetSystemLibrary.IsValidClass` (`self.CScene`))
    (bind _returnvalue (`|CreateWidget` "/Game/Blueprints/Text.Text_C" (`GameplayStatics.GetPlayerController` 0)))
    (bind _output_get (set `local.NewLocalVar` _returnvalue))
    (`UserWidget.AddToViewport` _output_get 0)
    (`Widget.SetVisibility` _output_get "Visible")
    (bind _returnvalue_2 (`|AddComponentByClass` (`self.CScene`)))
    (`/Game/Blueprints/NPC_cScene/CScene.Load` _returnvalue_2 _output_get)))

(fn `UserConstructionScript`)