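; BP_Statue is a collectible that jumps around the play area in the collection game mode.
; InitStatue teleports it to a random X/Y point at ground height and restarts a looping relocation timer whose interval shrinks as the game mode's Level rises.
; When the player character overlaps it before game over, it reports the collection to BP_GameMode_Collection, clears the timer and relocates at once.
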(event `self.ReceiveBeginPlay`
  (bind _asbp_game_mode_collection (cast `/Game/Blueprints/CollectionGame/BP_GameMode_Collection` (`GameplayStatics.GetGameMode`)))
  (set `self.gamemode` _asbp_game_mode_collection)
  (`self.InitStatue`))

(event `self.ReceiveActorBeginOverlap`
  (params (OtherActor :type "Actor Object Reference"))
  (bind _gamemode (`self.gamemode`))
  (if (and (== OtherActor (`GameplayStatics.GetPlayerCharacter` 0)) (not (`/Game/Blueprints/CollectionGame/BP_GameMode_Collection.GameOver` _gamemode)))
    (`/Game/Blueprints/CollectionGame/BP_GameMode_Collection.StatueCollected` _gamemode)
    (`KismetSystemLibrary.K2_ClearTimer` null "InitStatue")
    (`self.InitStatue`)))

(fn `InitStatue`
  (`self.K2_TeleportTo` (`KismetMathLibrary.MakeVector` (`KismetMathLibrary.RandomFloatInRange` -1800.0 1000.0) (`KismetMathLibrary.RandomFloatInRange` -1400.0 1400.0)))
  (`KismetSystemLibrary.K2_SetTimer` null "InitStatue" (/ 15.0 (`KismetMathLibrary.Conv_IntToDouble` (`/Game/Blueprints/CollectionGame/BP_GameMode_Collection.Level` (`self.gamemode`)))) true))

(fn `UserConstructionScript`)