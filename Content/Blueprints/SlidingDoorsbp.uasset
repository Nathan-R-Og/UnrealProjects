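; Sliding double door Blueprint that opens on trigger overlap and closes when the overlap ends, unless locked.
; A timeline, rate-scaled to Duration, lerps two frames in opposite directions along the Slide offset from their starting positions.
; The door registers itself as an owner on each key at BeginPlay.
; CheckKeysifChanged prunes invalid keys, unlocking when any is gone or, with AllRequired, when none remain.
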(event `self.ReceiveBeginPlay`
  (bind _door_driver (`self.door driver`))
  (bind _output_get (set `self.DoorAStart` (`SceneComponent.RelativeLocation` (`self.frame1`))))
  (bind _output_get_2 (set `self.DoorBStart` (`SceneComponent.RelativeLocation` (`self.frame2`))))
  (`TimelineComponent.SetPlayRate` _door_driver (/ (`TimelineComponent.GetTimelineLength` _door_driver) (`self.Duration`)))
  (for _array_element (`self.Keys`)
    (`KismetArrayLibrary.Array_Add` (`/Game/Blueprints/DoorKey.Owners` _array_element) self)))

(event `self.trigger.OnComponentBeginOverlap`
  (params (OverlappedComponent :type "PrimitiveComponent Object Reference") (OtherActor :type "Actor Object Reference") (OtherComp :type "PrimitiveComponent Object Reference") (OtherBodyIndex :type Integer) (bFromSweep :type Boolean) (SweepResult :type "HitResult Structure (by ref)"))
  (bind _slide (`self.Slide`))
  (if (not (`self.Locked`))
    (bind (_direction _driver) (`Timeline|door driver` :!label _label)
      (:`Update`
        (`SceneComponent.K2_SetRelativeLocation` (`self.frame1`) (`KismetMathLibrary.VLerp` (stale `self.ReceiveBeginPlay` _output_get) (+ (`KismetMathLibrary.NegateVector` _slide) (stale `self.ReceiveBeginPlay` _output_get)) _driver) false false)
        (`SceneComponent.K2_SetRelativeLocation` (`self.frame2`) (`KismetMathLibrary.VLerp` (stale `self.ReceiveBeginPlay` _output_get_2) (+ _slide (stale `self.ReceiveBeginPlay` _output_get_2)) _driver) false false)))))

(event `self.trigger.OnComponentEndOverlap`
  (params (OverlappedComponent :type "PrimitiveComponent Object Reference") (OtherActor :type "Actor Object Reference") (OtherComp :type "PrimitiveComponent Object Reference") (OtherBodyIndex :type Integer))
  (if (not (`self.Locked`))
    (goto _label :!via `Reverse`)))

(event `Check Keys if Changed`
  (bind _keys (`self.Keys`))
  (for (_array_element _array_index) _keys
    (if (== (`KismetSystemLibrary.IsValid` _array_element) false)
      (`KismetArrayLibrary.Array_Remove` _keys _array_index)
      (if (`self.AllRequired`)
        (set `self.Locked` (not (== (`KismetArrayLibrary.Array_Length` _keys) 0)))
        (else
          (set `self.Locked` false))))))

(fn `UserConstructionScript`)