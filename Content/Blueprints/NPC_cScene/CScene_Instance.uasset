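; CScene_Instance is an NPC cutscene script that plays hard-coded placeholder dialogue through a text object passed to it.
; Load stores that reference, sets an initial typing speed, initializes it with lines defined at runtime and binds OnInc to its next-line event.
; OnInc switches on the dialogue index to give later lines their own typing speed.
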(event `self.Load`
  (params (NewParam :type "/Game/Blueprints/Text Object Reference"))
  (set `self.TextReference` NewParam)
  (set `/Game/Blueprints/Text.typingSpeed` 5.0 NewParam)
  (`/Game/Blueprints/Text.Init` NewParam (`|MakeArray` "OOOOOooo this text is made at runtime ooo" "oooo this is a class not a actor varaible ooo" "this is so that i can instance this where i want ooo" "BOO!!!!!"))
  ;[1 1 1] silly
  (add `/Game/Blueprints/Text.Next` (`self.TextReference`) (delegate `OnInc`)))

(event `OnInc`
  (bind _textreference (`self.TextReference`))
  ;[1 1 1] silly
  (switch `int` (`/Game/Blueprints/Text.DIndex` _textreference)
    (:`1`
      (set `/Game/Blueprints/Text.typingSpeed` 0.001 _textreference))
    (:`2`
      (set `/Game/Blueprints/Text.typingSpeed` 0.154 _textreference))
    (:`3`
      (set `/Game/Blueprints/Text.typingSpeed` 0.05 _textreference))))