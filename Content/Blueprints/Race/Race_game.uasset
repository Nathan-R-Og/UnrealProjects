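; Race game logic Blueprint that starts a timed race when the level's Start actor is touched.
; On BeginPlay it finds the Start actor and binds to its Touched event, which calls StartGame.
; StartGame runs only if not already playing: it resets and starts the Timer, then has Race_Hud create a Start_Text widget and plays its Drop animation.
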(event `self.ReceiveBeginPlay`
  (bind _returnvalue (`GameplayStatics.GetActorOfClass` "/Game/Blueprints/Race/Start.Start_C"))
  (add `/Game/Blueprints/Race/Start.Touched` _returnvalue (delegate `Touched_Event`)))

(event `Touched_Event`
  (`self.StartGame`))

(fn `StartGame`
  (bind _timer (`self.Timer`))
  (if (not (`self.Playing`))
    (set `/Game/Blueprints/Timer.Time` 0.0 _timer)
    (set `/Game/Blueprints/Timer.Counting` true _timer)
    (set `self.Playing` true)
    (bind _asrace_hud (cast `/Game/Blueprints/Race/Race_Hud` (`PlayerController.GetHUD` (`GameplayStatics.GetPlayerController` 0))))
    (bind _give_class (`/Game/Blueprints/Race/Race_Hud.MakeMeWidget` _asrace_hud "/Game/Blueprints/Race/Start_Text.Start_Text_C"))
    (bind _asstart_text (cast `/Game/Blueprints/Race/Start_Text` _give_class))
    (`UserWidget.PlayAnimation` _asstart_text (`/Game/Blueprints/Race/Start_Text.drop` _asstart_text) 0.0 1 "Forward" 1.0 false)))

(fn `UserConstructionScript`)