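; Path runner actor that, while active, moves through a looping list of path point actors.
; Tick steps the root toward the current point at MoveSpeed, then a distance check advances the wrapped list index once within range.
; Direction changes turn the actor to face the point on the horizontal plane only.
; Movement runs only with HadDynamicDirection set, re-aiming every step, and uses no sweep.
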(event `self.ReceiveBeginPlay`
  (set `self.CurrentPoint` (`|GetArrayItem` (`self.PathList`)))
  (`self.SetMoveDirection`))

(event `self.ReceiveTick`
  (params (DeltaSeconds :type "Float (single-precision)"))
  (if (`self.IsActive`)
    (`self.MoveRunner` DeltaSeconds)
    (`self.CheckDistanceAndUpdate`)))

(fn `CheckDistanceAndUpdate`
  (bind _output_get (set `self.IsPointWIthinRange` (< (`KismetMathLibrary.VSize` (- (`SceneComponent.K2_GetComponentLocation` (`Actor.RootComponent` (`self.CurrentPoint`))) (`SceneComponent.K2_GetComponentLocation` (`self.DefaultSceneRoot`)))) (`self.PointWithinRange`))))
  (if _output_get
    (`self.NextPathPoint`)
    (`self.SetMoveDirection`)))

(fn `MoveRunner`
  (params (DeltaSeconds :type "Float (double-precision)"))
  (bind _defaultsceneroot (`self.DefaultSceneRoot`))
  (if (and (`self.HadDynamicDirection`) (not (`self.IsPointWIthinRange`)))
    (`self.SetMoveDirection`)
    (`SceneComponent.K2_SetWorldLocation` _defaultsceneroot (+ (`SceneComponent.K2_GetComponentLocation` _defaultsceneroot) (* DeltaSeconds (`self.MoveSpeed`) (`self.MoveDirection`))) false false)))

(fn `NextPathPoint`
  (bind _pathlist (`self.PathList`))
  (bind _result (`/Engine/EditorBlueprintResources/StandardMacros.IncrementInt` (`self.PathListIndex`))
    (:`  `
      (bind _result_2 (`/Engine/EditorBlueprintResources/StandardMacros.DecrementInt` (`KismetArrayLibrary.Array_Length` _pathlist))
        (:`  `
          (bind _returnvalue (`KismetMathLibrary.Wrap` _result -1 _result_2))
          (set `self.CurrentPoint` (`|GetArrayItem` _pathlist _returnvalue))
          (set `self.PathListIndex` _returnvalue))))))

(fn `SetMoveDirection`
  (locals (NewLocalVar :type "Rotator Structure" :default (struct)) (NewLocalVar_0 :type "Vector Structure"))
  (bind _defaultsceneroot (`self.DefaultSceneRoot`))
  (bind _output_get (set `local.NewLocalVar_0` (- (`SceneComponent.K2_GetComponentLocation` (`Actor.RootComponent` (`self.CurrentPoint`))) (`SceneComponent.K2_GetComponentLocation` _defaultsceneroot))))
  (set `self.MoveDirection` (`KismetMathLibrary.Normal` _output_get))
  (bind (_x _y) (`KismetMathLibrary.BreakVector3f` _output_get))
  (`SceneComponent.K2_SetRelativeRotation` _defaultsceneroot (`KismetMathLibrary.Conv_VectorToRotator` (`KismetMathLibrary.MakeVector` _x _y)) false false))

(fn `UserConstructionScript`)